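; BP_Cubey is a test-style trigger that counts up while the third person character stands inside its Box component.
; Begin and end overlap events set a status flag that gates the Tick logic.
; Tick alternates between a one-second Delay and incrementing then printing Number, using a completion flag to pace the count at roughly once per second.
; The count is never reset on exit.
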(event OnComponentBeginOverlap(Box)
  (params (OverlappedComponent :type Primitive%20Component%20Object%20Reference) (OtherActor :type Actor%20Object%20Reference) (OtherComp :type Primitive%20Component%20Object%20Reference) (OtherBodyIndex :type Integer) (bFromSweep :type Boolean) (SweepResult :type Hit%20Result%20Structure%20%28by%20ref%29))
  (if (== (Utilities|GetClass OtherActor) "/Game/ThirdPerson/Blueprints/BP_ThirdPersonCharacter.BP_ThirdPersonCharacter_C")
    (Variables|Default|SetOverlapStatus true)))

(event OnComponentEndOverlap(Box)
  (params (OverlappedComponent :type Primitive%20Component%20Object%20Reference) (OtherActor :type Actor%20Object%20Reference) (OtherComp :type Primitive%20Component%20Object%20Reference) (OtherBodyIndex :type Integer))
  (if (== (Utilities|GetClass OtherActor) "/Game/ThirdPerson/Blueprints/BP_ThirdPersonCharacter.BP_ThirdPersonCharacter_C")
    (Variables|Default|SetOverlapStatus false)))

(event EventTick
  (params (DeltaSeconds :type Float%20%28single-precision%29))
  (if (Variables|Default|GetOverlapStatus)
    (if (Variables|Default|GetHasCompletedDelay)
      (bind _result (Math|Integer|IncrementInt (Variables|Default|GetNumber))
        (:%20%20
          (bind _output_get (Variables|Default|SetNumber _result))
          (Development|PrintString (Utilities|String|ToString(Integer) _output_get))
          (Variables|Default|SetHasCompletedDelay false)))
      (else
        (Utilities|FlowControl|Delay 1.0)
        (Variables|Default|SetHasCompletedDelay true)))))

(fn ConstructionScript)